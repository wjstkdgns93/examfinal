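; Player hero Blueprint that moves relative to camera yaw and attacks by punching or firing a gun.
; Left click sets a punching flag, or starts and stops the gun when EatGun is true; the Gunset event spawns that gun onto GunSocket.
; BeginPlay shows the cursor and spawns a marker actor, which clicks move to the point under the cursor.
; The construction script attaches the two punch components to the hand sockets.
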(event `InputAxis|MoveForword`
  (params (AxisValue :type "Float (single-precision)"))
  (`self.AddMovementInput` (`KismetMathLibrary.GetForwardVector` (`KismetMathLibrary.MakeRotator` 0.0 0.0 (.yaw (`self.GetControlRotation`)))) AxisValue))

(event `InputAxis|MoveLeftRight`
  (params (AxisValue :type "Float (single-precision)"))
  (`self.AddMovementInput` (`KismetMathLibrary.GetRightVector` (`KismetMathLibrary.MakeRotator` 0.0 0.0 (.yaw (`self.GetControlRotation`)))) AxisValue))

(event `self.ReceiveBeginPlay`
  (bind _returnvalue (`|SpawnActorFromClass` "/Game/UI/MousePointBP.MousePointBP_C" (`KismetMathLibrary.Conv_VectorToTransform` (`self.K2_GetActorLocation`)) "Undefined" "OverrideRootScale"))
  (set `self.MouseClickPoint` _returnvalue)
  (set `PlayerController.bShowMouseCursor` true (`GameplayStatics.GetPlayerController` 0)))

(event `InputAction|LeftMouseClicked`
  (params (Key :type "Key Structure" :default "AnyKey"))
  (bind _gun (`self.Gun`))
  (bind _eatgun_ (`self.eatGun?`))
  (:`Pressed`
    (if _eatgun_
      (`/Game/BP/GunsetBP.StartFiring` _gun)
      (else
        (set `self.isPunching?` true))))
  (:`Released`
    (if _eatgun_
      (`/Game/BP/GunsetBP.StopFiring` _gun)
      (else
        (set `self.isPunching?` false)))))

(event `Gunset`
  (bind _returnvalue (`|SpawnActorFromClass` "/Game/BP/GunsetBP.GunsetBP_C" (`SceneComponent.K2_GetComponentToWorld` (`self.Mesh`)) "Undefined" "OverrideRootScale"))
  (bind _output_get (set `self.Gun` _returnvalue))
  (`self.K2_AttachToComponent` _output_get (`self.Mesh`) "GunSocket" "SnapToTarget" "SnapToTarget" "KeepWorld" true))

(event `InputAction|LeftMouseClicked`
  (params (Key :type "Key Structure" :default "AnyKey"))
  (:`Pressed`
    (`self.K2_SetActorLocation` (`self.MouseClickPoint`) (`.Location` (`GameplayStatics.BreakHitResult` (`PlayerController.GetHitResultUnderCursorByChannel` (`GameplayStatics.GetPlayerController` 0) "TraceTypeQuery1" true))) false false)))

(fn `UserConstructionScript`
  (bind _mesh (`self.Mesh`))
  (`SceneComponent.K2_AttachToComponent` (`self.RightPunch`) _mesh "hand_r" "SnapToTarget" "SnapToTarget" "KeepWorld" true)
  (`SceneComponent.K2_AttachToComponent` (`self.LeftPunch`) _mesh "hand_l" "SnapToTarget" "SnapToTarget" "KeepWorld" true))